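; Player character Blueprint that handles a simple crouch input and health-based death.
; Pressing Crouch shifts the whole actor down by a local offset, with no release handling to raise it again.
; Incoming damage reduces and prints Health, then calls OnDeath on BP_PlayerController once Health reaches zero or below.
; Leftover unconnected nodes include a duplicate offset and a grounded-movement velocity check.
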(event `InputAction|Crouch`
  (params (Key :type "Key Structure"))
  ;[1 1 1] Crouch
  (:`Pressed`
    (`self.K2_AddActorLocalOffset` (0.0 0.0 -30.0))))

(event `/Game/_Main/Blueprints/BPI_TakingDamage.TakeDamage`
  (params (Damage :type "Float (single-precision)"))
  ;[1 1 1] Player Death
  (bind _output_get (set `self.Health` (- (`self.Health`) Damage)))
  (`KismetSystemLibrary.PrintString` (`KismetStringLibrary.Conv_DoubleToString` _output_get))
  (if (<= _output_get 0.0)
    (bind _asbp_player_controller (cast `/Game/_Main/Blueprints/BP_PlayerController` (`self.GetController`)))
    (`/Game/_Main/Blueprints/BP_PlayerController.onDeath` _asbp_player_controller)))

(fn `UserConstructionScript`)